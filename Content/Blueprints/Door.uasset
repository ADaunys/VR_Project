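; VR door Blueprint that a motion controller swings open by its handle, with a lock tied to a Keyhole.
; Grab stores the controller as Hand when it is within the handle's collision sphere, and Release clears it.
; Each Tick locks the door only while fully closed and the Keyhole is not unlocked.
; An unlocked door yaws toward the held hand within clamped world-space limits, or snaps shut when released nearly closed.
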(event EventTick
  (params (DeltaSeconds :type Float%20%28single-precision%29))
  (bind _hand (Variables|Default|GetHand))
  (bind _door (Variables|Default|GetDoor))
  (Utilities|FlowControl|Sequence
    (:then_0
      ;[1 1 1] Is Locked
      (if (and (not (Variables|/Game/Blueprints/KeyHole.KeyHole_C|GetUnlocked (Variables|Default|GetKeyhole))) (Math|Float|NearlyEqual(Float) (.yaw (Transformation|GetWorldRotation (Variables|Default|GetDoor))) 0.0 1e-06))
        (Variables|Default|SetLocked true)
        (else
          (Variables|Default|SetLocked false))))
    (:then_1
      ;[1 1 1] Set Door Rotation
      (if (not (Variables|Default|GetLocked))
        (Utilities|IsValid _hand
          (:Is%20Valid
            (Transformation|SetWorldRotation _door (Math|Rotator|MakeRotator 0.0 0.0 (Math|Float|ClampAngle (- (.yaw (Math|Rotator|FindLookatRotation (Transformation|GetWorldLocation _hand) (Transformation|GetWorldLocation _door))) 9e+01) -9e+01 9e+01)) false false))
          (:Is%20Not%20Valid
            (if (Math|Float|NearlyEqual(Float) (.yaw (Transformation|GetWorldRotation _door)) 0.0 1e+01)
              (Transformation|SetWorldRotation _door "0, 0, 0" false false))))))))

(event EventGrab
  (params (MotionController :type Motion%20Controller%20Component%20Object%20Reference))
  (bind _handlecollision (Variables|Default|GetHandleCollision))
  (if (Utilities|Operators|EqualEqual (Transformation|GetWorldLocation MotionController) (Transformation|GetWorldLocation _handlecollision) (Variables|/Script/Engine.SphereComponent|GetSphereRadius _handlecollision))
    (Variables|Default|SetHand MotionController)))

(event EventRelease
  (params (MotionController :type Motion%20Controller%20Component%20Object%20Reference))
  (if (== MotionController (Variables|Default|GetHand))
    (Variables|Default|SetHand 0)))

(fn ConstructionScript)