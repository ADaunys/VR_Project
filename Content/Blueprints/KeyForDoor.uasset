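; KeyForDoor is a key actor that motion controllers can grab and release, with no door logic in this graph.
; Release clears the controller reference, detaches the actor in world space and re-enables mesh physics.
; Grab only clears the reference after an equality check, while a separate custom event stores the controller.
; The nodes that snap-attach to the controller and disable physics are disconnected, so they never run.
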(event Custom|CustomEvent
  (params (MotionController :type Motion%20Controller%20Component%20Object%20Reference))
  (Variables|Default|SetMotion%20Controller MotionController))

(event EventTick
  (params (DeltaSeconds :type Float%20%28single-precision%29)))

(event EventRelease
  (params (MotionController :type Motion%20Controller%20Component%20Object%20Reference))
  (Variables|Default|SetMotion%20Controller 0)
  (Transformation|DetachFromActor "KeepWorld" "KeepWorld" "KeepWorld")
  (Physics|SetSimulatePhysics (Variables|Default|GetKeyMesh) true))

(event EventGrab
  (params (MotionController :type Motion%20Controller%20Component%20Object%20Reference))
  (if (== MotionController (Variables|Default|GetMotion%20Controller))
    (Variables|Default|SetMotion%20Controller 0)))

(fn ConstructionScript)