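; VR orb puzzle Blueprint in which a grabbed motion controller turns the top ring.
; Grab and Release store and clear the controller; while it is valid, Tick calls a macro that sets RingTop's yaw from a look-at toward the controller's position in ring-relative space.
; AllRingsAligned unhides OrbTop, but nothing here detects alignment; a yaw-range visibility check is left disconnected.
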(event Custom|AllRingsAligned
  (Development|SetHiddeninGame (Variables|Default|GetOrbTop) false false))

(event EventBeginPlay)

(event Collision|EventActorBeginOverlap
  (params (OtherActor :type Actor%20Object%20Reference)))

(event EventGrab
  (params (MotionController :type Motion%20Controller%20Component%20Object%20Reference))
  (Variables|Default|SetMotion%20Controller MotionController))

(event EventRelease
  (params (MotionController :type Motion%20Controller%20Component%20Object%20Reference))
  (if (== MotionController (Variables|Default|GetMotion%20Controller))
    (Variables|Default|SetMotion%20Controller 0)))

(event EventTick
  (params (DeltaSeconds :type Float%20%28single-precision%29))
  (bind _ring_top (Variables|Default|GetRing%20Top))
  (bind _motion_controller (Variables|Default|GetMotion%20Controller)
    (:then
      (Utilities|NewMacro1 _ring_top _ring_top _ring_top _motion_controller))
    (:else)))

(fn ConstructionScript)